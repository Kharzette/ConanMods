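; Shared item Blueprint for alchemy elixirs that alter a player's sex, body proportions, face or voice.
; On use, the server adds corruption through BPEnergyReceiver, then picks the effect by TemplateID.
; Effects rebuild the CharacterLayout through OnCharacterLayoutChanged, clamping height and physique, while sex-mismatched elixirs apply a buff instead.
; Voice helpers use if-chains to map or cycle the non-contiguous voice enum, and voice changes show a notification.
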(event `self.OnUseItem`
  (params (invokingCharacter :type "ConanCharacter Object Reference"))
  (bind _returnvalue (`Actor.K2_GetComponentsByClass` invokingCharacter "/Game/Systems/BPEnergyReceiver.BPEnergyReceiver_C"))
  (bind _templateid (`self.TemplateID`))
  (`parent.OnUseItem` invokingCharacter)
  (if (`Actor.HasAuthority` invokingCharacter)
    (bind _asbase_player_char (cast `/Game/Characters/BasePlayerChar` invokingCharacter))
    ;[1 1 1] Add some corruption... wanted to max out at an amount, but not sure what a max should be, gets kind of buggy
    (if (> (`KismetArrayLibrary.Array_Length` _returnvalue) 0)
      (`EnergyReceiverComponent.ModifyEnergy` (`KismetArrayLibrary.Array_Get` _returnvalue) "EnergyType_Corruption" 50.0)
      (if (== _templateid 54153001)
        (`self.MakeFemale` _asbase_player_char)
        (elif (== _templateid 54153002)
          (`self.MakeMale` _asbase_player_char)
          (elif (== _templateid 54153003)
            (`self.ChangeBoobs` _asbase_player_char 0.1)
            (elif (== _templateid 54153004)
              (`self.ChangeBoobs` _asbase_player_char -0.1)
              (elif (== _templateid 54153005)
                (`self.ChangeDong` _asbase_player_char -0.1)
                (elif (== _templateid 54153006)
                  (`self.ChangeDong` _asbase_player_char 0.1)
                  (elif (== _templateid 54153008)
                    (`self.ChangeHeight` _asbase_player_char 0.05)
                    (elif (== _templateid 54153009)
                      (`self.ChangeHeight` _asbase_player_char -0.05)
                      (elif (== _templateid 54153010)
                        (`self.ChangeFace` _asbase_player_char)
                        (elif (== _templateid 54153011)
                          (`self.ChangeVoice` _asbase_player_char)
                          (elif (== _templateid 54153016)
                            (`self.ChangePhysique` _asbase_player_char 0.1)
                            (elif (== _templateid 54153017)
                              (`self.ChangePhysique` _asbase_player_char -0.1))))))))))))))))

(fn `AdvanceVoiceIndex`
  (params (voiceIdx :type Integer))
  (returns (retIdx :type Integer))
  (bind _returnvalue (cast `/Game/Sound/Tables/VoiceSetType` (`KismetMathLibrary.Conv_IntToByte` voiceIdx)))
  ;[1 1 1] Fun with non contiguous enums, default is erroneously assigned sometimes
  (if (`|EnumEquality` _returnvalue "NewEnumerator70")
    (return (`KismetMathLibrary.Conv_ByteToInt` (enumliteral `/Game/Sound/Tables/VoiceSetType` "NewEnumerator0")))
    (elif (`|EnumEquality` _returnvalue "NewEnumerator0")
      (return (`KismetMathLibrary.Conv_ByteToInt` (enumliteral `/Game/Sound/Tables/VoiceSetType` "NewEnumerator1")))
      (elif (`|EnumEquality` _returnvalue "NewEnumerator1")
        (return (`KismetMathLibrary.Conv_ByteToInt` (enumliteral `/Game/Sound/Tables/VoiceSetType` "NewEnumerator2")))
        (elif (`|EnumEquality` _returnvalue "NewEnumerator2")
          (return (`KismetMathLibrary.Conv_ByteToInt` (enumliteral `/Game/Sound/Tables/VoiceSetType` "NewEnumerator3")))
          (elif (`|EnumEquality` _returnvalue "NewEnumerator3")
            (return (`KismetMathLibrary.Conv_ByteToInt` (enumliteral `/Game/Sound/Tables/VoiceSetType` "NewEnumerator4")))
            (elif (`|EnumEquality` _returnvalue "NewEnumerator4")
              (return (`KismetMathLibrary.Conv_ByteToInt` (enumliteral `/Game/Sound/Tables/VoiceSetType` "NewEnumerator49")))
              (elif (`|EnumEquality` _returnvalue "NewEnumerator49")
                (return (`KismetMathLibrary.Conv_ByteToInt` (enumliteral `/Game/Sound/Tables/VoiceSetType` "NewEnumerator0")))
                (elif (`|EnumEquality` _returnvalue "NewEnumerator5")
                  (return (`KismetMathLibrary.Conv_ByteToInt` (enumliteral `/Game/Sound/Tables/VoiceSetType` "NewEnumerator6")))
                  (elif (`|EnumEquality` _returnvalue "NewEnumerator6")
                    (return (`KismetMathLibrary.Conv_ByteToInt` (enumliteral `/Game/Sound/Tables/VoiceSetType` "NewEnumerator7")))
                    (elif (`|EnumEquality` _returnvalue "NewEnumerator7")
                      (return (`KismetMathLibrary.Conv_ByteToInt` (enumliteral `/Game/Sound/Tables/VoiceSetType` "NewEnumerator8")))
                      (elif (`|EnumEquality` _returnvalue "NewEnumerator8")
                        (return (`KismetMathLibrary.Conv_ByteToInt` (enumliteral `/Game/Sound/Tables/VoiceSetType` "NewEnumerator9")))
                        (elif (`|EnumEquality` _returnvalue "NewEnumerator9")
                          (return (`KismetMathLibrary.Conv_ByteToInt` (enumliteral `/Game/Sound/Tables/VoiceSetType` "NewEnumerator50")))
                          (elif (`|EnumEquality` _returnvalue "NewEnumerator50")
                            (return (`KismetMathLibrary.Conv_ByteToInt` (enumliteral `/Game/Sound/Tables/VoiceSetType` "NewEnumerator5")))
                            (else
                              (return -1))))))))))))))))

(fn `ChangeBoobs`
  (params (playerChar :type "/Game/Characters/BasePlayerChar Object Reference") (amount :type "Float (double-precision)"))
  (bind _character_layout (`/Game/Characters/BasePlayerChar.GetCharacterLayout` playerChar))
  (bind (_meshlayout _texturelayout _tintlayout _boolparams _intparams _scalarparams _enumparams _armourdyeparams) (break `CharacterLayout` _character_layout))
  ;[1 1 1] This potion isn't for men
  (if (`.IsFemale` (break `CharacterBoolParameters` _boolparams))
    (bind (_height _bust _dick _eyeangle _eyesize _eyedepth _nosewidth _nosesize _nosecurve _jawwidth _cheekheight _cheekwidth _chinwidth _earangle _earsize _lipsize _pitch _physiquemax _physiquemin) (break `CharacterScalarParameters` _scalarparams))
    (`/Game/Characters/BasePlayerChar.OnCharacterLayoutChanged` playerChar (make `CharacterLayout` _meshlayout _texturelayout _tintlayout _boolparams _intparams (make `CharacterScalarParameters` _height (+ _bust amount) _dick _eyeangle _eyesize _eyedepth _nosewidth _nosesize _nosecurve _jawwidth _cheekheight _cheekwidth _chinwidth _earangle _earsize _lipsize _pitch _physiquemax _physiquemin) _enumparams _armourdyeparams))
    (else
      (`/Game/Systems/Buffs/00_BP_AC_BuffSystem.AddBuff` (`/Game/Characters/BaseBPCombat.00_BP_AC_BuffSystem` playerChar) "/Game/Mods/Alchemy2/BluePrints/Not4MaleBuff.Not4MaleBuff_C" playerChar 69 (`/Game/Characters/FuncomFunctionLibrary.GetControllerFromActor` playerChar)))))

(fn `ChangeDong`
  (params (playerChar :type "/Game/Characters/BasePlayerChar Object Reference") (amount :type "Float (double-precision)"))
  (bind _character_layout (`/Game/Characters/BasePlayerChar.GetCharacterLayout` playerChar))
  (bind (_meshlayout _texturelayout _tintlayout _boolparams _intparams _scalarparams _enumparams _armourdyeparams) (break `CharacterLayout` _character_layout))
  ;[1 1 1] This potion isn't for ladies
  (if (`.IsFemale` (break `CharacterBoolParameters` _boolparams))
    (`/Game/Systems/Buffs/00_BP_AC_BuffSystem.AddBuff` (`/Game/Characters/BaseBPCombat.00_BP_AC_BuffSystem` playerChar) "/Game/Mods/Alchemy2/BluePrints/Not4FemaleBuff.Not4FemaleBuff_C" playerChar 69 (`/Game/Characters/FuncomFunctionLibrary.GetControllerFromActor` playerChar))
    (else
      (bind (_height _bust _dick _eyeangle _eyesize _eyedepth _nosewidth _nosesize _nosecurve _jawwidth _cheekheight _cheekwidth _chinwidth _earangle _earsize _lipsize _pitch _physiquemax _physiquemin) (break `CharacterScalarParameters` _scalarparams))
      (`/Game/Characters/BasePlayerChar.OnCharacterLayoutChanged` playerChar (make `CharacterLayout` _meshlayout _texturelayout _tintlayout _boolparams _intparams (make `CharacterScalarParameters` _height _bust (+ _dick amount) _eyeangle _eyesize _eyedepth _nosewidth _nosesize _nosecurve _jawwidth _cheekheight _cheekwidth _chinwidth _earangle _earsize _lipsize _pitch _physiquemax _physiquemin) _enumparams _armourdyeparams)))))

(fn `ChangeFace`
  (params (playerChar :type "/Game/Characters/BasePlayerChar Object Reference"))
  (bind _character_layout (`/Game/Characters/BasePlayerChar.GetCharacterLayout` playerChar))
  (bind (_meshlayout _texturelayout _tintlayout _boolparams _intparams _scalarparams _enumparams _armourdyeparams) (break `CharacterLayout` _character_layout))
  (if (`.IsFemale` (break `CharacterBoolParameters` _boolparams))
    (bind (_helmet _hair _facialhair _head _forearms _hands _upperbody _lowerbody _legs _feet) (break `CharacterMeshLayout` _meshlayout))
    (`/Game/Characters/BasePlayerChar.OnCharacterLayoutChanged` playerChar (make `CharacterLayout` (make `CharacterMeshLayout` _helmet _hair _facialhair (mod (+ _head 1) (`CharacterFunctionLibrary.LengthDataTable` "/Game/UI/CharacterCreation/DataTables/Female_HeadSelections.Female_HeadSelections")) _forearms _hands _upperbody _lowerbody _legs _feet) _texturelayout _tintlayout _boolparams _intparams _scalarparams _enumparams _armourdyeparams))
    (else
      (bind (_meshlayout_2 _texturelayout_2 _tintlayout_2 _boolparams_2 _intparams_2 _scalarparams_2 _enumparams_2 _armourdyeparams_2) (break `CharacterLayout` _character_layout))
      (bind (_helmet_2 _hair_2 _facialhair_2 _head_2 _forearms_2 _hands_2 _upperbody_2 _lowerbody_2 _legs_2 _feet_2) (break `CharacterMeshLayout` _meshlayout_2))
      (`/Game/Characters/BasePlayerChar.OnCharacterLayoutChanged` playerChar (make `CharacterLayout` (make `CharacterMeshLayout` _helmet_2 _hair_2 _facialhair_2 (mod (+ _head_2 1) (`CharacterFunctionLibrary.LengthDataTable` "/Game/UI/CharacterCreation/DataTables/Male_HeadSelections.Male_HeadSelections")) _forearms_2 _hands_2 _upperbody_2 _lowerbody_2 _legs_2 _feet_2) _texturelayout_2 _tintlayout_2 _boolparams_2 _intparams_2 _scalarparams_2 _enumparams_2 _armourdyeparams_2)))))

(fn `ChangeHeight`
  (params (playerChar :type "/Game/Characters/BasePlayerChar Object Reference") (amount :type "Float (double-precision)"))
  (bind _character_layout (`/Game/Characters/BasePlayerChar.GetCharacterLayout` playerChar))
  (bind (_meshlayout _texturelayout _tintlayout _boolparams _intparams _scalarparams _enumparams _armourdyeparams) (break `CharacterLayout` _character_layout))
  (bind (_height _bust _dick _eyeangle _eyesize _eyedepth _nosewidth _nosesize _nosecurve _jawwidth _cheekheight _cheekwidth _chinwidth _earangle _earsize _lipsize _pitch _physiquemax _physiquemin) (break `CharacterScalarParameters` _scalarparams))
  (`/Game/Characters/BasePlayerChar.OnCharacterLayoutChanged` playerChar (make `CharacterLayout` _meshlayout _texturelayout _tintlayout _boolparams _intparams (make `CharacterScalarParameters` (`KismetMathLibrary.FClamp` (+ _height amount) 0.75 1.25) _bust _dick _eyeangle _eyesize _eyedepth _nosewidth _nosesize _nosecurve _jawwidth _cheekheight _cheekwidth _chinwidth _earangle _earsize _lipsize _pitch _physiquemax _physiquemin) _enumparams _armourdyeparams)))

(fn `ChangePhysique`
  (params (playerChar :type "/Game/Characters/BasePlayerChar Object Reference") (amount :type "Float (double-precision)"))
  (bind _character_layout (`/Game/Characters/BasePlayerChar.GetCharacterLayout` playerChar))
  (bind (_meshlayout _texturelayout _tintlayout _boolparams _intparams _scalarparams _enumparams _armourdyeparams) (break `CharacterLayout` _character_layout))
  (bind (_height _bust _dick _eyeangle _eyesize _eyedepth _nosewidth _nosesize _nosecurve _jawwidth _cheekheight _cheekwidth _chinwidth _earangle _earsize _lipsize _pitch _physiquemax _physiquemin) (break `CharacterScalarParameters` _scalarparams))
  (`/Game/Characters/BasePlayerChar.OnCharacterLayoutChanged` playerChar (make `CharacterLayout` _meshlayout _texturelayout _tintlayout _boolparams _intparams (make `CharacterScalarParameters` _height _bust _dick _eyeangle _eyesize _eyedepth _nosewidth _nosesize _nosecurve _jawwidth _cheekheight _cheekwidth _chinwidth _earangle _earsize _lipsize _pitch (`KismetMathLibrary.FMin` (`KismetMathLibrary.FMax` (+ _physiquemax amount) 0.0) 1.0) (`KismetMathLibrary.FMin` (`KismetMathLibrary.FMax` (+ _physiquemin amount) 0.0) 1.0)) _enumparams _armourdyeparams)))

(fn `ChangeVoice`
  (params (playerChar :type "/Game/Characters/BasePlayerChar Object Reference"))
  (locals (voiceIdx :type Integer))
  (bind _character_layout (`/Game/Characters/BasePlayerChar.GetCharacterLayout` playerChar))
  (bind (_meshlayout _texturelayout _tintlayout _boolparams _intparams _scalarparams _enumparams _armourdyeparams) (break `CharacterLayout` _character_layout))
  (bind (_physique _voice) (break `CharacterIntParameters` _intparams))
  ;[1 1 1] Check for and fix invalid values
  (if (<= _voice 0)
    (if (`.IsFemale` (break `CharacterBoolParameters` _boolparams))
      (set `local.voiceIdx` (`KismetMathLibrary.Conv_ByteToInt` (enumliteral `/Game/Sound/Tables/VoiceSetType` "NewEnumerator5")))
      (else
        (set `local.voiceIdx` (`KismetMathLibrary.Conv_ByteToInt` (enumliteral `/Game/Sound/Tables/VoiceSetType` "NewEnumerator0")))))
    (else
      (set `local.voiceIdx` _voice)))
  (bind _retidx (`self.AdvanceVoiceIndex` (`local.voiceIdx`)))
  (`/Game/Characters/BasePlayerChar.OnCharacterLayoutChanged` playerChar (make `CharacterLayout` _meshlayout _texturelayout _tintlayout _boolparams (make `CharacterIntParameters` _physique _retidx) _scalarparams _enumparams _armourdyeparams))
  (`self.SpewTextForNewVoice` (`local.voiceIdx`) (`/Game/Characters/FuncomFunctionLibrary.GetControllerFromActor` playerChar)))

(fn `ConvertVoiceIndex`
  (params (voiceIdx :type Integer))
  (returns (retIdx :type Integer))
  (bind _returnvalue (cast `/Game/Sound/Tables/VoiceSetType` (`KismetMathLibrary.Conv_IntToByte` voiceIdx)))
  ;[1 1 1] Fun with non contiguous enums
  (if (`|EnumEquality` _returnvalue "NewEnumerator70")
    (return (`KismetMathLibrary.Conv_ByteToInt` (enumliteral `/Game/Sound/Tables/VoiceSetType` "NewEnumerator5")))
    (elif (`|EnumEquality` _returnvalue "NewEnumerator0")
      (return (`KismetMathLibrary.Conv_ByteToInt` (enumliteral `/Game/Sound/Tables/VoiceSetType` "NewEnumerator5")))
      (elif (`|EnumEquality` _returnvalue "NewEnumerator1")
        (return (`KismetMathLibrary.Conv_ByteToInt` (enumliteral `/Game/Sound/Tables/VoiceSetType` "NewEnumerator6")))
        (elif (`|EnumEquality` _returnvalue "NewEnumerator2")
          (return (`KismetMathLibrary.Conv_ByteToInt` (enumliteral `/Game/Sound/Tables/VoiceSetType` "NewEnumerator7")))
          (elif (`|EnumEquality` _returnvalue "NewEnumerator3")
            (return (`KismetMathLibrary.Conv_ByteToInt` (enumliteral `/Game/Sound/Tables/VoiceSetType` "NewEnumerator8")))
            (elif (`|EnumEquality` _returnvalue "NewEnumerator4")
              (return (`KismetMathLibrary.Conv_ByteToInt` (enumliteral `/Game/Sound/Tables/VoiceSetType` "NewEnumerator9")))
              (elif (`|EnumEquality` _returnvalue "NewEnumerator49")
                (return (`KismetMathLibrary.Conv_ByteToInt` (enumliteral `/Game/Sound/Tables/VoiceSetType` "NewEnumerator50")))
                (elif (`|EnumEquality` _returnvalue "NewEnumerator5")
                  (return (`KismetMathLibrary.Conv_ByteToInt` (enumliteral `/Game/Sound/Tables/VoiceSetType` "NewEnumerator0")))
                  (elif (`|EnumEquality` _returnvalue "NewEnumerator6")
                    (return (`KismetMathLibrary.Conv_ByteToInt` (enumliteral `/Game/Sound/Tables/VoiceSetType` "NewEnumerator1")))
                    (elif (`|EnumEquality` _returnvalue "NewEnumerator7")
                      (return (`KismetMathLibrary.Conv_ByteToInt` (enumliteral `/Game/Sound/Tables/VoiceSetType` "NewEnumerator2")))
                      (elif (`|EnumEquality` _returnvalue "NewEnumerator8")
                        (return (`KismetMathLibrary.Conv_ByteToInt` (enumliteral `/Game/Sound/Tables/VoiceSetType` "NewEnumerator3")))
                        (elif (`|EnumEquality` _returnvalue "NewEnumerator9")
                          (return (`KismetMathLibrary.Conv_ByteToInt` (enumliteral `/Game/Sound/Tables/VoiceSetType` "NewEnumerator4")))
                          (elif (`|EnumEquality` _returnvalue "NewEnumerator50")
                            (return (`KismetMathLibrary.Conv_ByteToInt` (enumliteral `/Game/Sound/Tables/VoiceSetType` "NewEnumerator49")))
                            (else
                              (return -1))))))))))))))))

(fn `MakeFemale`
  (params (playerChar :type "/Game/Characters/BasePlayerChar Object Reference"))
  (locals (voiceSet :type Integer))
  (bind _character_layout (`/Game/Characters/BasePlayerChar.GetCharacterLayout` playerChar))
  (bind (_meshlayout _texturelayout _tintlayout _boolparams _intparams _scalarparams _enumparams _armourdyeparams) (break `CharacterLayout` _character_layout))
  ;[1 1 1] This potion isn't for ladies
  (if (`.IsFemale` (break `CharacterBoolParameters` _boolparams))
    (`/Game/Systems/Buffs/00_BP_AC_BuffSystem.AddBuff` (`/Game/Characters/BaseBPCombat.00_BP_AC_BuffSystem` playerChar) "/Game/Mods/Alchemy2/BluePrints/Not4FemaleBuff.Not4FemaleBuff_C" playerChar 69 (`/Game/Characters/FuncomFunctionLibrary.GetControllerFromActor` playerChar))
    (else
      ;[1 1 1] Make sure the voice set is in the female range
      (bind _retidx (`self.ConvertVoiceIndex` (`.Voice` (break `CharacterIntParameters` (`.IntParams` (break `CharacterLayout` _character_layout))))))
      (set `local.voiceSet` _retidx)
      (bind (_helmet _hair _facialhair _head _forearms _hands _upperbody _lowerbody _legs _feet) (break `CharacterMeshLayout` _meshlayout))
      (`/Game/Characters/BasePlayerChar.OnCharacterLayoutChanged` playerChar (make `CharacterLayout` (make `CharacterMeshLayout` _helmet _hair 0 _head _forearms _hands _upperbody _lowerbody _legs _feet) _texturelayout _tintlayout (make `CharacterBoolParameters` true) (make `CharacterIntParameters` (`.Physique` (break `CharacterIntParameters` _intparams)) (`local.voiceSet`)) (make `CharacterScalarParameters` (`.Height` (break `CharacterScalarParameters` _scalarparams)) 1.0 1.0 0.73 1.08 -0.002 0.04 0.95 -5.3 0.25 0.0 -0.17 1.53 0.0 1.0 0.0 1.0) _enumparams _armourdyeparams)))))

(fn `MakeMale`
  (params (playerChar :type "/Game/Characters/BasePlayerChar Object Reference"))
  (locals (voiceSet :type Integer))
  (bind _character_layout (`/Game/Characters/BasePlayerChar.GetCharacterLayout` playerChar))
  (bind (_meshlayout _texturelayout _tintlayout _boolparams _intparams _scalarparams _enumparams _armourdyeparams) (break `CharacterLayout` _character_layout))
  ;[1 1 1] This potion isn't for men
  (if (`.IsFemale` (break `CharacterBoolParameters` _boolparams))
    ;[1 1 1] Make sure the voice set is in the male range
    (bind _retidx (`self.ConvertVoiceIndex` (`.Voice` (break `CharacterIntParameters` (`.IntParams` (break `CharacterLayout` _character_layout))))))
    (set `local.voiceSet` _retidx)
    (`/Game/Characters/BasePlayerChar.OnCharacterLayoutChanged` playerChar (make `CharacterLayout` _meshlayout _texturelayout _tintlayout (make `CharacterBoolParameters` false) (make `CharacterIntParameters` (`.Physique` (break `CharacterIntParameters` _intparams)) (`local.voiceSet`)) _scalarparams _enumparams _armourdyeparams))
    (`self.ChangeFace` playerChar)
    (else
      (`/Game/Systems/Buffs/00_BP_AC_BuffSystem.AddBuff` (`/Game/Characters/BaseBPCombat.00_BP_AC_BuffSystem` playerChar) "/Game/Mods/Alchemy2/BluePrints/Not4MaleBuff.Not4MaleBuff_C" playerChar 69 (`/Game/Characters/FuncomFunctionLibrary.GetControllerFromActor` playerChar)))))

(fn `SpewTextForNewVoice`
  (params (voiceIdx :type Integer) (playerController :type "Controller Object Reference"))
  (bind _returnvalue (cast `/Game/Sound/Tables/VoiceSetType` (`KismetMathLibrary.Conv_IntToByte` voiceIdx)))
  (if (`|EnumEquality` _returnvalue "NewEnumerator70")
    (message `/Game/Characters/HUDNotification_Interface.NotificationText` playerController "You feel mute..." true :!label _label)
    (elif (`|EnumEquality` _returnvalue "NewEnumerator0")
      (message `/Game/Characters/HUDNotification_Interface.NotificationText` playerController "You feel Strong!" true)
      (elif (`|EnumEquality` _returnvalue "NewEnumerator1")
        (message `/Game/Characters/HUDNotification_Interface.NotificationText` playerController "You feel Stoic!" true)
        (elif (`|EnumEquality` _returnvalue "NewEnumerator2")
          (message `/Game/Characters/HUDNotification_Interface.NotificationText` playerController "You feel Desperate!" true)
          (elif (`|EnumEquality` _returnvalue "NewEnumerator3")
            (message `/Game/Characters/HUDNotification_Interface.NotificationText` playerController "You feel Learned!" true)
            (elif (`|EnumEquality` _returnvalue "NewEnumerator4")
              (message `/Game/Characters/HUDNotification_Interface.NotificationText` playerController "You feel Grim!" true)
              (elif (`|EnumEquality` _returnvalue "NewEnumerator49")
                (message `/Game/Characters/HUDNotification_Interface.NotificationText` playerController "You feel Excited!" true)
                (elif (`|EnumEquality` _returnvalue "NewEnumerator5")
                  (message `/Game/Characters/HUDNotification_Interface.NotificationText` playerController "You feel Strong!" true)
                  (elif (`|EnumEquality` _returnvalue "NewEnumerator6")
                    (message `/Game/Characters/HUDNotification_Interface.NotificationText` playerController "You feel Desperate!" true)
                    (elif (`|EnumEquality` _returnvalue "NewEnumerator7")
                      (message `/Game/Characters/HUDNotification_Interface.NotificationText` playerController "You feel Savage!" true)
                      (elif (`|EnumEquality` _returnvalue "NewEnumerator8")
                        (message `/Game/Characters/HUDNotification_Interface.NotificationText` playerController "You feel Jubilant!" true)
                        (elif (`|EnumEquality` _returnvalue "NewEnumerator9")
                          (message `/Game/Characters/HUDNotification_Interface.NotificationText` playerController "You feel Manic!" true)
                          (elif (`|EnumEquality` _returnvalue "NewEnumerator50")
                            (message `/Game/Characters/HUDNotification_Interface.NotificationText` playerController "You feel like a Berserker!" true)
                            (else
                              (`LoggerLibrary.DWLogString` "Big if chain found nothing" "Network" "INFOL_IMPORTANT")
                              (goto _label))))))))))))))))