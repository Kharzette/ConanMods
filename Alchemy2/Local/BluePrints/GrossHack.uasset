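; GrossHack is a component on BasePlayerChar that plays client-side feedback for grooming actions like tweezing, scissors, shaving, lip paint and mascara.
; Client-named events play a 2D sound, and the grooming ones also play a borrowed emote or combat montage.
; PlayGenderMontage picks montages from the character layout's IsFemale flag, but plays MaleAnim when it is true.
; Other events play a learn sound or forward notification text to the owner's controller.
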(event `self.ReceiveBeginPlay`
  (bind _asbase_player_char (cast `/Game/Characters/BasePlayerChar` (`self.GetOwner`)))
  (set `self.MyCharacter` _asbase_player_char))

(event `ClientPlayLearnSound`
  (`GameplayStatics.PlaySound2D` "/Game/Mods/Alchemy2/Assets/FeatLearny.FeatLearny"))

(event `ClientPlayTweezerSound`
  (`GameplayStatics.PlaySound2D` "/Game/Sound/SFX/Weapons/Bow_Crossbow/sfx_crossbow_fire_1.sfx_crossbow_fire_1")
  (`self.PlayTweezeAnim`))

(event `ClientPlayScissorSound`
  (`GameplayStatics.PlaySound2D` "/Game/Sound/SFX/Doors/Traps/Spike_Trap/spike_trap_retract_1.spike_trap_retract_1")
  (`self.PlayScissorAnim`))

(event `ClientPlayShavingSound`
  (`GameplayStatics.PlaySound2D` "/Game/Sound/SFX/Doors/Traps/Spike_Trap/spike_trap_retract_1.spike_trap_retract_1")
  (`self.PlayShaveAnim`))

(event `ClientPlayLipPaintSound`
  (`GameplayStatics.PlaySound2D` "/Game/Sound/SFX/Impacts/Soft_Impact/impact_soft_1.impact_soft_1")
  (`self.PlayLipAnim`))

(event `ClientPlayMascaraSound`
  (`GameplayStatics.PlaySound2D` "/Game/Sound/SFX/Impacts/Soft_Impact/impact_soft_Normal.impact_soft_Normal")
  (`self.PlayMascaraAnim`))

(event `ClientNotify`
  (params (NotificationText :type String) (bPositive :type Boolean))
  (message `/Game/Characters/HUDNotification_Interface.NotificationText` (`/Game/Characters/FuncomFunctionLibrary.GetControllerFromActor` (`self.MyCharacter`)) (`KismetTextLibrary.Conv_StringToText` NotificationText) bPositive))

(fn `PlayGenderMontage`
  (params (MaleAnim :type "AnimMontage Object Reference") (FemaleAnim :type "AnimMontage Object Reference"))
  (bind _mycharacter (`self.MyCharacter`))
  (bind _character_layout (`/Game/Characters/BasePlayerChar.GetCharacterLayout` (`self.MyCharacter`)))
  (if (`.IsFemale` (break `CharacterBoolParameters` (`.BoolParams` (break `CharacterLayout` _character_layout))))
    (`Character.PlayAnimMontage` _mycharacter MaleAnim 1.0 "None")
    (else
      (`Character.PlayAnimMontage` _mycharacter FemaleAnim 1.0 "None"))))

(fn `PlayLipAnim`
  (`self.PlayGenderMontage` "/Game/Characters/humans/animations/emotes/AM_emote_blow_kiss_m.AM_emote_blow_kiss_m" "/Game/Characters/humans/animations/emotes/AM_emote_blow_kiss_f.AM_emote_blow_kiss_f"))

(fn `PlayMascaraAnim`
  (`self.PlayGenderMontage` "/Game/Characters/humans/animations/emotes/AM_emote_fist_punch_m.AM_emote_fist_punch_m" "/Game/Characters/humans/animations/emotes/AM_emote_show_off_f.AM_emote_show_off_f"))

(fn `PlayScissorAnim`
  (`self.PlayGenderMontage` "/Game/Characters/humans/animations/emotes/AM_emote_comb_hair_m.AM_emote_comb_hair_m" "/Game/Characters/humans/animations/emotes/AM_emote_comb_hair_f.AM_emote_comb_hair_f"))

(fn `PlayShaveAnim`
  (`self.PlayGenderMontage` "/Game/Characters/humans/animations/emotes/AM_emote_ponder_m.AM_emote_ponder_m" "/Game/Characters/humans/animations/emotes/AM_emote_shrug_m.AM_emote_shrug_m"))

(fn `PlayTweezeAnim`
  (`self.PlayGenderMontage` "/Game/Characters/humans/animations/combat/knockbacks/AM_combat_gethit_SS.AM_combat_gethit_SS" "/Game/Characters/humans/animations/combat/knockbacks/AM_combat_gethit_SS.AM_combat_gethit_SS"))