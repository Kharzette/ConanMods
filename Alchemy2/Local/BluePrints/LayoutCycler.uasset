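; Usable grooming item that advances one cosmetic of the user's character, with the feature picked by item TemplateID (scissors, shaving kit, kohl brush, lip paint, tweezers).
; On the server, it rebuilds the character layout with that index incremented, wrapping at the length of the matching, mostly gender-specific, data table.
; Facial hair only changes for males and lip paint for females.
; Each successful change plays a client sound through the character's GrossHack component.
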(event `self.OnUseItem`
  (params (invokingCharacter :type "ConanCharacter Object Reference"))
  (bind _templateid (`self.TemplateID`))
  (`parent.OnUseItem` invokingCharacter)
  (if (`KismetSystemLibrary.IsServer`)
    (bind _asbase_player_char (cast `/Game/Characters/BasePlayerChar` invokingCharacter))
    ;[1 1 1] Which item am I?
    (if (== _templateid 54153007)
      (bind _returnvalue (`Actor.GetComponentByClass` _asbase_player_char "/Game/Mods/Alchemy2/BluePrints/GrossHack.GrossHack_C"))
      (`self.CycleLayoutElement` _asbase_player_char "NewEnumerator0" _returnvalue)
      (elif (== _templateid 54153012)
        (`self.CycleLayoutElement` _asbase_player_char "NewEnumerator1" _returnvalue)
        (elif (== _templateid 54153013)
          (`self.CycleLayoutElement` _asbase_player_char "NewEnumerator4" _returnvalue)
          (elif (== _templateid 54153014)
            (`self.CycleLayoutElement` _asbase_player_char "NewEnumerator3" _returnvalue)
            (elif (== _templateid 54153015)
              (`self.CycleLayoutElement` _asbase_player_char "NewEnumerator2" _returnvalue))))))))

(fn `CanUseItem`
  (params (invokingCharacter :type "ConanCharacter Object Reference"))
  (returns (ReturnValue :type Boolean))
  (return true))

(fn `CycleBrows`
  (params (Character :type "/Game/Characters/BasePlayerChar Object Reference") (bFemale :type Boolean) (ClientStuff :type "/Game/Mods/Alchemy2/BluePrints/GrossHack Object Reference"))
  (locals (ModBy :type Integer))
  (bind _character_layout (`/Game/Characters/BasePlayerChar.GetCharacterLayout` Character))
  (if bFemale
    (set `local.ModBy` (`CharacterFunctionLibrary.LengthDataTable` "/Game/UI/CharacterCreation/DataTables/Female_EyebrowSelections.Female_EyebrowSelections"))
    (else
      (set `local.ModBy` (`CharacterFunctionLibrary.LengthDataTable` "/Game/UI/CharacterCreation/DataTables/Male_EyebrowSelections.Male_EyebrowSelections"))))
  (bind (_meshlayout _texturelayout _tintlayout _boolparams _intparams _scalarparams _enumparams _armourdyeparams) (break `CharacterLayout` _character_layout))
  (bind (_eyebrowtexture _eyetexture _liptexture _warpaintfacetexture _warpaintbodytexture _warpainthandstexture _hairlinetexture _facialhairlinetexture) (break `CharacterTextureLayout` _texturelayout))
  (`/Game/Characters/BasePlayerChar.OnCharacterLayoutChanged` Character (make `CharacterLayout` _meshlayout (make `CharacterTextureLayout` (mod (+ _eyebrowtexture 1) (`local.ModBy`)) _eyetexture _liptexture _warpaintfacetexture _warpaintbodytexture _warpainthandstexture _hairlinetexture _facialhairlinetexture) _tintlayout _boolparams _intparams _scalarparams _enumparams _armourdyeparams))
  (`/Game/Mods/Alchemy2/BluePrints/GrossHack.ClientPlayTweezerSound` ClientStuff))

(fn `CycleEyeMakeUp`
  (params (Character :type "/Game/Characters/BasePlayerChar Object Reference") (bFemale :type Boolean) (ClientStuff :type "/Game/Mods/Alchemy2/BluePrints/GrossHack Object Reference"))
  (locals (ModBy :type Integer))
  (bind _character_layout (`/Game/Characters/BasePlayerChar.GetCharacterLayout` Character))
  (if bFemale
    (set `local.ModBy` (`CharacterFunctionLibrary.LengthDataTable` "/Game/UI/CharacterCreation/DataTables/Female_EyesSelections.Female_EyesSelections"))
    (else
      (set `local.ModBy` (`CharacterFunctionLibrary.LengthDataTable` "/Game/UI/CharacterCreation/DataTables/Male_EyesSelections.Male_EyesSelections"))))
  (bind (_meshlayout _texturelayout _tintlayout _boolparams _intparams _scalarparams _enumparams _armourdyeparams) (break `CharacterLayout` _character_layout))
  (bind (_eyebrowtexture _eyetexture _liptexture _warpaintfacetexture _warpaintbodytexture _warpainthandstexture _hairlinetexture _facialhairlinetexture) (break `CharacterTextureLayout` _texturelayout))
  (`/Game/Characters/BasePlayerChar.OnCharacterLayoutChanged` Character (make `CharacterLayout` _meshlayout (make `CharacterTextureLayout` _eyebrowtexture (mod (+ _eyetexture 1) (`local.ModBy`)) _liptexture _warpaintfacetexture _warpaintbodytexture _warpainthandstexture _hairlinetexture _facialhairlinetexture) _tintlayout _boolparams _intparams _scalarparams _enumparams _armourdyeparams))
  (`/Game/Mods/Alchemy2/BluePrints/GrossHack.ClientPlayMascaraSound` ClientStuff))

(fn `CycleFacialHair`
  (params (Character :type "/Game/Characters/BasePlayerChar Object Reference") (bFemale :type Boolean) (ClientStuff :type "/Game/Mods/Alchemy2/BluePrints/GrossHack Object Reference"))
  (bind _character_layout (`/Game/Characters/BasePlayerChar.GetCharacterLayout` Character))
  (if (not bFemale)
    (bind (_meshlayout _texturelayout _tintlayout _boolparams _intparams _scalarparams _enumparams _armourdyeparams) (break `CharacterLayout` _character_layout))
    (bind (_helmet _hair _facialhair _head _forearms _hands _upperbody _lowerbody _legs _feet) (break `CharacterMeshLayout` _meshlayout))
    (`/Game/Characters/BasePlayerChar.OnCharacterLayoutChanged` Character (make `CharacterLayout` (make `CharacterMeshLayout` _helmet _hair (mod (+ _facialhair 1) (`CharacterFunctionLibrary.LengthDataTable` "/Game/UI/CharacterCreation/DataTables/FacialHairStyleTable.FacialHairStyleTable")) _head _forearms _hands _upperbody _lowerbody _legs _feet) _texturelayout _tintlayout _boolparams _intparams _scalarparams _enumparams _armourdyeparams))
    (`/Game/Mods/Alchemy2/BluePrints/GrossHack.ClientPlayShavingSound` ClientStuff)))

(fn `CycleHair`
  (params (Character :type "/Game/Characters/BasePlayerChar Object Reference") (bFemale :type Boolean) (ClientStuff :type "/Game/Mods/Alchemy2/BluePrints/GrossHack Object Reference"))
  (locals (ModBy :type Integer))
  (bind _character_layout (`/Game/Characters/BasePlayerChar.GetCharacterLayout` Character))
  (if bFemale
    (set `local.ModBy` (`CharacterFunctionLibrary.LengthDataTable` "/Game/UI/CharacterCreation/DataTables/Female_HairStyleSelections.Female_HairStyleSelections"))
    (else
      (set `local.ModBy` (`CharacterFunctionLibrary.LengthDataTable` "/Game/UI/CharacterCreation/DataTables/Male_HairStyleSelections.Male_HairStyleSelections"))))
  (bind (_meshlayout _texturelayout _tintlayout _boolparams _intparams _scalarparams _enumparams _armourdyeparams) (break `CharacterLayout` _character_layout))
  (bind (_helmet _hair _facialhair _head _forearms _hands _upperbody _lowerbody _legs _feet) (break `CharacterMeshLayout` _meshlayout))
  (`/Game/Characters/BasePlayerChar.OnCharacterLayoutChanged` Character (make `CharacterLayout` (make `CharacterMeshLayout` _helmet (mod (+ _hair 1) (`local.ModBy`)) _facialhair _head _forearms _hands _upperbody _lowerbody _legs _feet) _texturelayout _tintlayout _boolparams _intparams _scalarparams _enumparams _armourdyeparams))
  (`/Game/Mods/Alchemy2/BluePrints/GrossHack.ClientPlayScissorSound` ClientStuff))

(fn `CycleLayoutElement`
  (params (Character :type "/Game/Characters/BasePlayerChar Object Reference") (choice :type "/Game/Mods/Alchemy2/BluePrints/LayoutChoices Enum") (ClientStuff :type "/Game/Mods/Alchemy2/BluePrints/GrossHack Object Reference"))
  (bind _character_layout (`/Game/Characters/BasePlayerChar.GetCharacterLayout` Character))
  (switch `/Game/Mods/Alchemy2/BluePrints/LayoutChoices` choice
    (:`NewEnumerator0`
      (bind _isfemale (break `CharacterBoolParameters` (`.BoolParams` (break `CharacterLayout` _character_layout))))
      (`self.CycleHair` Character _isfemale ClientStuff))
    (:`NewEnumerator1`
      (`self.CycleFacialHair` Character _isfemale ClientStuff))
    (:`NewEnumerator2`
      (`self.CycleBrows` Character _isfemale ClientStuff))
    (:`NewEnumerator4`
      (`self.CycleEyeMakeUp` Character _isfemale ClientStuff))
    (:`NewEnumerator3`
      (`self.CycleLipMakeUp` Character _isfemale ClientStuff))))

(fn `CycleLipMakeUp`
  (params (Character :type "/Game/Characters/BasePlayerChar Object Reference") (bFemale :type Boolean) (ClientStuff :type "/Game/Mods/Alchemy2/BluePrints/GrossHack Object Reference"))
  (bind _character_layout (`/Game/Characters/BasePlayerChar.GetCharacterLayout` Character))
  (if bFemale
    (bind (_meshlayout _texturelayout _tintlayout _boolparams _intparams _scalarparams _enumparams _armourdyeparams) (break `CharacterLayout` _character_layout))
    (bind (_eyebrowtexture _eyetexture _liptexture _warpaintfacetexture _warpaintbodytexture _warpainthandstexture _hairlinetexture _facialhairlinetexture) (break `CharacterTextureLayout` _texturelayout))
    (`/Game/Characters/BasePlayerChar.OnCharacterLayoutChanged` Character (make `CharacterLayout` _meshlayout (make `CharacterTextureLayout` _eyebrowtexture _eyetexture (mod (+ _liptexture 1) (`CharacterFunctionLibrary.LengthDataTable` "/Game/UI/CharacterCreation/DataTables/Female_LipsSelections.Female_LipsSelections")) _warpaintfacetexture _warpaintbodytexture _warpainthandstexture _hairlinetexture _facialhairlinetexture) _tintlayout _boolparams _intparams _scalarparams _enumparams _armourdyeparams))
    (`/Game/Mods/Alchemy2/BluePrints/GrossHack.ClientPlayLipPaintSound` ClientStuff)))