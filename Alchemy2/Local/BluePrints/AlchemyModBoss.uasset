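; Mod controller for the Alchemy2 mod that injects its content into the game's data tables.
; ModDataTableOperations merges new items, compounds, feats and recipes, then adds alchemy book pages to tiered misc loot, including Highlands variants.
; It also merges name-to-template mappings and resource loot changes to put alchemy components into rare harvests.
; Two Tier 3/4 plunder merges show no target table; all other graphs are empty.
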(fn `ModDataTableOperations`
  ;[1 1 1] New Items
  (`self.MergeDataTables` "/Game/Items/ItemTable.ItemTable" "/Game/Mods/Alchemy2/Tables/NewItems.NewItems")
  (`self.MergeDataTables` "/Game/Items/ItemTable.ItemTable" "/Game/Mods/Alchemy2/Tables/AlchemyCompounds.AlchemyCompounds")
  ;[1 1 1] New Feats & Recipes
  (`self.MergeDataTables` "/Game/Items/Feats/FeatTable.FeatTable" "/Game/Mods/Alchemy2/Tables/NewFeats.NewFeats")
  (`self.MergeDataTables` "/Game/Items/Recipes/RecipesTable.RecipesTable" "/Game/Mods/Alchemy2/Tables/NewRecipes.NewRecipes")
  ;[1 1 1] Adjust alchemy book pages into the misc loot
  (`self.MergeDataTables` "/Game/Systems/Loot/TableSetup/W_T1MiscLoot.W_T1MiscLoot" "/Game/Mods/Alchemy2/Tables/NewPlunderT1.NewPlunderT1")
  (`self.MergeDataTables` "/Game/Systems/Loot/TableSetup/W_T2MiscLoot.W_T2MiscLoot" "/Game/Mods/Alchemy2/Tables/NewPlunderT2.NewPlunderT2")
  (`self.MergeDataTables` "/Game/Systems/Loot/TableSetup/W_T3MiscLoot.W_T3MiscLoot" "/Game/Mods/Alchemy2/Tables/NewPlunderT3.NewPlunderT3")
  (`self.MergeDataTables` "/Game/Systems/Loot/TableSetup/W_T4MiscLoot.W_T4MiscLoot" "/Game/Mods/Alchemy2/Tables/NewPlunderT4.NewPlunderT4")
  ;[1 1 1] Highlands
  (`self.MergeDataTables` "/Game/Systems/Loot/TableSetup/W_T3MiscLoot_Highlands.W_T3MiscLoot_Highlands" "/Game/Mods/Alchemy2/Tables/NewPlunderT3.NewPlunderT3")
  (`self.MergeDataTables` "/Game/Systems/Loot/TableSetup/W_T4MiscLoot_Highlands.W_T4MiscLoot_Highlands" "/Game/Mods/Alchemy2/Tables/NewPlunderT4.NewPlunderT4")
  (`self.MergeDataTables` null "/Game/Mods/Alchemy2/Tables/NewPlunderT3.NewPlunderT3")
  (`self.MergeDataTables` null "/Game/Mods/Alchemy2/Tables/NewPlunderT4.NewPlunderT4")
  ;[1 1 1] Put alchemy components into rare harvests
  (`self.MergeDataTables` "/Game/Systems/Survival/Gathering/Gathering_v2/ItemNameToTemplateID.ItemNameToTemplateID" "/Game/Mods/Alchemy2/Tables/MyNameToTemplate.MyNameToTemplate")
  (`self.MergeDataTables` "/Game/Systems/Survival/Gathering/Gathering_v2/LootTable_Resource.LootTable_Resource" "/Game/Mods/Alchemy2/Tables/ResourceTableMods.ResourceTableMods"))

(fn `UserConstructionScript`)