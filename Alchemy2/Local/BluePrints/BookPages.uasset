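; Usable item Blueprint for alchemy book pages that teach the using character an alchemy feat.
; On use, the server maps the page's template ID to a feat ID through a branch chain and checks the character's progression system.
; Known feats trigger a negative notification; new ones play a sound, notify, force-learn the feat and call the parent use handler.
; Client feedback routes through the GrossHack component, and Yellow Lotus currently clears learned feats.
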(event `self.OnUseItem`
  (params (invokingCharacter :type "ConanCharacter Object Reference"))
  (bind _returnvalue (`Actor.GetComponentByClass` invokingCharacter "/Game/Mods/Alchemy2/BluePrints/GrossHack.GrossHack_C"))
  (bind _templateid (`self.TemplateID`))
  (if (`KismetSystemLibrary.IsServer`)
    ;[1 1 1] Which page am I?
    (if (== _templateid 54130001)
      (set `self.FeatID` 54150001)
      ;[1 1 1] Already have the feat?
      (bind _returnvalue_2 (`ConanCharacter.GetProgressionSystem` invokingCharacter :!label _label))
      (if (`ProgressionSystem.IsFeatPurchased` _returnvalue_2 (`self.FeatID`))
        (`/Game/Mods/Alchemy2/BluePrints/GrossHack.ClientNotify` _returnvalue "This knowledge is already yours" false)
        (else
          ;[1 1 1] Learn Feat, right now these are cleared by Yellow Lotus, but want to make them permanent eventually with the from npc flag
          (`/Game/Mods/Alchemy2/BluePrints/GrossHack.ClientPlayLearnSound` _returnvalue)
          (`/Game/Mods/Alchemy2/BluePrints/GrossHack.ClientNotify` _returnvalue "Alchemical secrets revealed!" true)
          (bind _returnvalue_3 (`ConanCharacter.GetProgressionSystem` invokingCharacter))
          (`ProgressionSystem.ServerForceLearnFeat` _returnvalue_3 (`self.FeatID`) false)
          (`parent.OnUseItem` invokingCharacter)))
      (elif (== _templateid 54130002)
        (set `self.FeatID` 54150003)
        (goto _label)
        (elif (== _templateid 54130003)
          (set `self.FeatID` 54150002)
          (goto _label)
          (elif (== _templateid 54130004)
            (set `self.FeatID` 54150004)
            (goto _label)
            (elif (== _templateid 54130005)
              (set `self.FeatID` 54150005)
              (goto _label))))))))